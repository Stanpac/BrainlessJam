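; Character that collects actors entering its DangerZone and can throw them back off.
; Overlapping actors have the touched component's collision disabled, snap onto the mesh and join a list, each lowering SpeedFactor by a fraction based on NbrOfActorToLose.
; Launch detaches the first listed BP_TestPawn, fires it along the character's forward vector and restores that fraction, gated by a cooldown.
; The construction script limits DangerZone to overlapping the Pawn channel.
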(event `self.DangerZone.OnComponentBeginOverlap`
  (params (OverlappedComponent :type "PrimitiveComponent Object Reference") (OtherActor :type "Actor Object Reference") (OtherComp :type "PrimitiveComponent Object Reference") (OtherBodyIndex :type Integer) (bFromSweep :type Boolean) (SweepResult :type "HitResult Structure (by ref)"))
  (if (!= OtherActor self)
    (`KismetArrayLibrary.Array_AddUnique` (`self.ActorAttatchToPlayer`) OtherActor)
    (`PrimitiveComponent.SetCollisionEnabled` OtherComp "NoCollision")
    (`self.K2_AttachToComponent` OtherActor (`self.Mesh`) "None" "SnapToTarget" "SnapToTarget" "SnapToTarget" true)
    (set `self.SpeedFactor` (`KismetMathLibrary.FClamp` (- (`self.SpeedFactor`) (`KismetMathLibrary.SafeDivide` 1.0 (`self.NbrOfActorToLose`)))))))

(event `self.Launch`
  (params (Value :type "InputActionValue Structure (by ref)"))
  (if (and (`KismetArrayLibrary.Array_IsNotEmpty` (`self.ActorAttatchToPlayer`)) (`self.CanUseLaunch`))
    (set `self.CanUseLaunch` false)
    (bind _asbp_test_pawn (cast `/Game/Blueprints/IA/BP_TestPawn` (`|GetArrayItem` (`self.ActorAttatchToPlayer`))))
    (`self.K2_DetachFromActor` _asbp_test_pawn "KeepWorld" "KeepWorld" "KeepWorld")
    (`KismetArrayLibrary.Array_RemoveItem` (`self.ActorAttatchToPlayer`) _asbp_test_pawn)
    (`/Game/Blueprints/IA/BP_TestPawn.Launch` _asbp_test_pawn (`self.GetActorForwardVector`))
    (set `self.SpeedFactor` (`KismetMathLibrary.FClamp` (+ (`self.SpeedFactor`) (`KismetMathLibrary.SafeDivide` 1.0 (`self.NbrOfActorToLose`)))))
    (`KismetSystemLibrary.Delay` (`self.LaunchCooldown`))
    (set `self.CanUseLaunch` true)))

(fn `UserConstructionScript`
  (`PrimitiveComponent.SetCollisionResponseToAllChannels` (`self.DangerZone`) "ECR_Ignore")
  (`PrimitiveComponent.SetCollisionResponseToChannel` (`self.DangerZone`) "ECC_Pawn" "ECR_Overlap"))